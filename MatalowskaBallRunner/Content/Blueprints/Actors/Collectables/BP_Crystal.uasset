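; BP_Crystal is a collectable crystal actor that flies to the player and vanishes when the player pawn enters its sphere.
; On overlap it records its starting location, scale and light intensity, then plays the TL_BlendAlpha timeline.
; Separate timeline tracks lerp it toward the player's live position, shrink it to zero and fade its point light.
; The actor destroys itself when the timeline finishes.
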(event OnComponentBeginOverlap(Sphere)
  (params (OverlappedComponent :type Primitive%20Component%20Object%20Reference) (OtherActor :type Actor%20Object%20Reference) (OtherComp :type Primitive%20Component%20Object%20Reference) (OtherBodyIndex :type Integer) (bFromSweep :type Boolean) (SweepResult :type Hit%20Result%20Structure%20%28by%20ref%29))
  (if (== OtherActor (Game|Player|GetPlayerPawn 0))
    (CallFunction|Crystal'sStartValues)
    (bind (_direction _smoothlerpalpha _scalechange _lightintensity) (Timeline|TL_BlendAlpha Play)
      (:Update
        (CallFunction|MoveCrystaltoPlayer _smoothlerpalpha)
        (CallFunction|ChangeCrystalScale _scalechange)
        (Rendering|Components|Light|SetIntensity (Variables|Default|GetPointLight) (Math|Float|Lerp (Variables|Default|GetLerpStartLightIntensity) 0.0 _lightintensity)))
      (:Finished
        (Actor|DestroyActor)))))

(event EventBeginPlay)

(event Collision|EventActorBeginOverlap
  (params (OtherActor :type Actor%20Object%20Reference)))

(event EventTick
  (params (DeltaSeconds :type Float%20%28single-precision%29)))

(fn ConstructionScript)

(fn MoveCrystaltoPlayer
  (params (Alpha :type Float%20%28single-precision%29))
  (Transformation|SetActorLocation (Math|Vector|Lerp(Vector) (Variables|Default|GetLerpStartLocation) (Transformation|GetActorLocation (Game|Player|GetPlayerPawn 0)) Alpha) false false))

(fn Crystal'sStartValues
  (Variables|Default|SetLerpStartLocation (Transformation|GetActorLocation))
  (Variables|Default|SetLerpStartScale (Transformation|GetActorScale3D))
  (Variables|Default|SetLerpStartLightIntensity (Variables|/Script/Engine.LightComponentBase|GetIntensity (Variables|Default|GetPointLight))))

(fn ChangeCrystalScale
  (params (Alpha :type Float%20%28single-precision%29))
  (Transformation|SetActorScale3D (Math|Vector|Lerp(Vector) (Variables|Default|GetLerpStartScale) "0, 0, 0" Alpha)))